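; Pedestrian-style traffic light actor that endlessly cycles red, steady green, then blinking green with a two-digit countdown, starting on BeginPlay.
; Delay-chained custom events run the timed phases, blinking green once per counted second until the counter ends and the cycle restarts.
; Helper events swap LED materials and toggle matching point lights; digits use a "Number" material parameter, blanking a leading zero.
; The construction script previews the starting Count through dynamic material instances.
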(event Custom|Red_Light
  (params (Red_Light_On :type Boolean))
  ;[1 0.2378 0.2378] Red_Light
  (Rendering|Material|SetMaterial (Variables|Default|Get신호등_LED_빨강) 0 (select Red_Light_On "/Game/01_Assets/09_TrafficLight/준비물/머티리얼/M_LED_RED.M_LED_RED" "/Game/01_Assets/09_TrafficLight/준비물/머티리얼/M_LED.M_LED"))
  (Rendering|SetVisibility (Variables|Default|GetPointLight_RED) Red_Light_On false))

(event Custom|Green_Light
  (params (Green_Light_On :type Boolean))
  ;[0.305 1 0.3038] Green_Light
  (Rendering|Material|SetMaterial (Variables|Default|Get신호등_LED_녹색) 0 (select Green_Light_On "/Game/01_Assets/09_TrafficLight/준비물/머티리얼/M_LED_GREEN.M_LED_GREEN" "/Game/01_Assets/09_TrafficLight/준비물/머티리얼/M_LED.M_LED"))
  (Rendering|SetVisibility (Variables|Default|GetPointLight_GREEN) Green_Light_On false))

(event Custom|Counter_Light
  (params (Counter_Light_On :type Boolean) (Counter :type Integer))
  ;[1 0.9174 0] Counter_Light
  (Rendering|Material|SetMaterial (Variables|Default|Get신호등_숫자LED_10) 0 (select Counter_Light_On "/Game/01_Assets/09_TrafficLight/준비물/머티리얼/M_LEDNUMBER.M_LEDNUMBER" "/Game/01_Assets/09_TrafficLight/준비물/머티리얼/M_LED.M_LED"))
  (Rendering|SetVisibility (Variables|Default|GetPointLight_COUNTER) Counter_Light_On false)
  (Rendering|Material|SetScalarParameterValueonMaterials (Variables|Default|Get신호등_숫자LED_1) "Number" (Math|Conversions|ToFloat(Integer) (Math|Integer|%(Integer) Counter 10)))
  (Rendering|Material|SetScalarParameterValueonMaterials (Variables|Default|Get신호등_숫자LED_10) "Number" (Math|Conversions|ToFloat(Integer) (/ Counter 10)))
  (if (< Counter 10)
    (Rendering|Material|SetMaterial (Variables|Default|Get신호등_숫자LED_10) 0 "/Game/01_Assets/09_TrafficLight/준비물/머티리얼/M_LED.M_LED")))

(event Custom|Initialize_Traffic_Light
  (CallFunction|RedLight false)
  (CallFunction|GreenLight false)
  (CallFunction|CounterLight false))

(event Custom|Traffic_Light_Loop
  (CallFunction|InitializeTrafficLight)
  ;[1 1 1] 빨간 라이트
  (CallFunction|RedLight true)
  (Utilities|FlowControl|Delay (Variables|Default|GetRed_Light_Duration))
  (CallFunction|RedLight false)
  ;[1 1 1] 초록 라이트
  (CallFunction|GreenLight true)
  (Utilities|FlowControl|Delay (Variables|Default|GetGreen_Light_Duration))
  (CallFunction|GreenLight false)
  ;[1 1 1] Counter_Loop
  (Variables|Default|SetCurrent_Count (+ (Variables|Default|GetCount) 1))
  (bind _result (Math|Integer|DecrementInt (Variables|Default|GetCurrent_Count))
    (:%20%20
      (CallFunction|CounterLight true _result)
      (CallFunction|GreenLight true)
      (Utilities|FlowControl|Delay 0.5)
      (CallFunction|GreenLight false)
      (Utilities|FlowControl|Delay 0.5)
      (if (< (Variables|Default|GetCurrent_Count) 2)
        (CallFunction|TrafficLightLoop)
        (else
          (CallFunction|CounterLoop))))))

(event Custom|Counter_Loop
  ;[1 1 1] Counter_Loop
  (bind _result (Math|Integer|DecrementInt (Variables|Default|GetCurrent_Count))
    (:%20%20
      (CallFunction|CounterLight true _result)
      (CallFunction|GreenLight true)
      (Utilities|FlowControl|Delay 0.5)
      (CallFunction|GreenLight false)
      (Utilities|FlowControl|Delay 0.5)
      (if (< (Variables|Default|GetCurrent_Count) 2)
        (CallFunction|TrafficLightLoop)
        (else
          (CallFunction|CounterLoop))))))

(event EventBeginPlay
  (CallFunction|TrafficLightLoop))

(fn ConstructionScript
  (bind _count (Variables|Default|GetCount))
  (bind _returnvalue (Rendering|Material|CreateDynamicMaterialInstance (Variables|Default|Get신호등_숫자LED_1) 0 "/Game/01_Assets/09_TrafficLight/준비물/머티리얼/M_LEDNUMBER.M_LEDNUMBER" "None" :!class /Script/Engine.PrimitiveComponent))
  (Rendering|Material|SetScalarParameterValue _returnvalue "Number" (Math|Conversions|ToFloat(Integer) (Math|Integer|%(Integer) _count 10)) :!class /Script/Engine.MaterialInstanceDynamic) ; 1의 자리
  (bind _returnvalue_2 (Rendering|Material|CreateDynamicMaterialInstance (Variables|Default|Get신호등_숫자LED_10) 0 (select (not (< _count 10)) "/Game/01_Assets/09_TrafficLight/준비물/머티리얼/M_LEDNUMBER.M_LEDNUMBER" "/Game/01_Assets/09_TrafficLight/준비물/머티리얼/M_LED.M_LED") "None" :!class /Script/Engine.PrimitiveComponent))
  (Rendering|Material|SetScalarParameterValue _returnvalue_2 "Number" (Math|Conversions|ToFloat(Integer) (/ _count 10)) :!class /Script/Engine.MaterialInstanceDynamic) ; 10의 자리
)