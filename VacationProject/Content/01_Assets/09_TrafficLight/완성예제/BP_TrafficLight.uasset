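; Pedestrian traffic light Blueprint that loops from BeginPlay through red, steady green and a blinking-green countdown.
; Delay nodes time each phase, and the countdown ticks about once per second before restarting the cycle.
; Setter events toggle point lights and swap emissive materials for each lamp and the counter.
; The counter splits the number into two digit meshes via a "Number" material parameter, blanking the tens below ten.
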(event Custom|Start%20Traffic%20Light
  ;[0.5654 0.6811 1] 신호등 흐름
  (CallFunction|Initialize)
  (CallFunction|SetRedLight true)
  (Utilities|FlowControl|Delay (Variables|Default|GetRed%20Light%20Duration))
  (CallFunction|SetRedLight false)
  (CallFunction|SetGreenLight true)
  (Utilities|FlowControl|Delay (Variables|Default|GetGreen%20Light%20Duration))
  (Variables|Default|SetCurrent%20Count (+ (Variables|Default|GetCount) 1))
  (bind _result (Math|Integer|DecrementInt (Variables|Default|GetCurrent%20Count) :!label _label)
    (:%20%20
      (if (> _result 0)
        (CallFunction|SetCounter true (Variables|Default|GetCurrent%20Count))
        (CallFunction|SetGreenLight true)
        (Utilities|FlowControl|Delay 0.5)
        (CallFunction|SetGreenLight false)
        (Utilities|FlowControl|Delay 0.5)
        (goto _label)
        (else
          ;;[0 0 0 1 12] 카운터 반복 탈출
          (CallFunction|StartTrafficLight))))))

(event Custom|Set%20Green%20Light
  (params (On :type Boolean))
  ;[0.5268 1 0.2531] 초록불 On / Off 하는 이벤트
  (Rendering|SetVisibility (Variables|Default|GetPointLight_GreenMark) On false)
  (Rendering|Material|SetMaterial (Variables|Default|GetTL_Human_3wayMirror_GreenLight_EM) 0 (select On "/Game/01_Assets/09_TrafficLight/완성예제/material/Light/MI_Emissive_Green.MI_Emissive_Green" "/Game/01_Assets/09_TrafficLight/완성예제/material/Light/M_Emissive_Off.M_Emissive_Off")))

(event Custom|Initialize
  ;[0.4271 0.4241 0.1478] 초기화. 모든 불을 끈다.
  (CallFunction|SetRedLight false)
  (CallFunction|SetGreenLight false)
  (CallFunction|SetCounter false))

(event Custom|Set%20Counter
  (params (On :type Boolean) (Number :type Integer))
  ;[0.3061 1 0.5856] 숫자 On / Off 그리고 숫자 설정해주는 이벤트
  (Rendering|SetVisibility (Variables|Default|GetPointLight_Counter) On false)
  (Rendering|Material|SetMaterial (Variables|Default|GetTL_Human_CounterLED_Mesh) 0 (select On "/Game/01_Assets/09_TrafficLight/완성예제/material/Light/M_Emissive_Num_On.M_Emissive_Num_On" "/Game/01_Assets/09_TrafficLight/완성예제/material/Light/M_Emissive_Num_Off.M_Emissive_Num_Off"))
  ;[0.3333 1 1] 불이 켜져있다면 숫자 설정
  (if On
    (Rendering|Material|SetScalarParameterValueonMaterials (Variables|Default|GetTL_Human_CounterLED_Mesh) "Number" (Math|Conversions|ToFloat(Integer) (/ Number 10)))
    (Rendering|Material|SetScalarParameterValueonMaterials (Variables|Default|GetTL_Human_CounterLED_Mesh1) "Number" (Math|Conversions|ToFloat(Integer) (Math|Integer|%(Integer) Number 10)))
    ;[0.4169 0.5979 1] 10 이하라면 10의자리 불 꺼주기
    (if (< Number 10)
      (Rendering|Material|SetMaterial (Variables|Default|GetTL_Human_CounterLED_Mesh) 0 "/Game/01_Assets/09_TrafficLight/완성예제/material/Light/M_Emissive_Num_Off.M_Emissive_Num_Off"))))

(event Custom|Count%20Loop
  ;[0.5654 0.6811 1] 신호등 흐름
  ;;[0 0 0 1 12] 카운터 이벤트 진입
  (bind _result (Math|Integer|DecrementInt (Variables|Default|GetCurrent%20Count) :!label _label)
    (:%20%20
      (if (> _result 0)
        (CallFunction|SetCounter true (Variables|Default|GetCurrent%20Count))
        (CallFunction|SetGreenLight true)
        (Utilities|FlowControl|Delay 0.5)
        (CallFunction|SetGreenLight false)
        (Utilities|FlowControl|Delay 0.5)
        (goto _label)
        (else
          ;;[0 0 0 1 12] 카운터 반복 탈출
          (CallFunction|StartTrafficLight))))))

(event Custom|Set%20Red%20Light
  (params (On :type Boolean))
  ;[1 0.228 0.2678] 빨간불 On / Off 하는 이벤트
  (Rendering|SetVisibility (Variables|Default|GetPointLight_RedMark) On false)
  (Rendering|Material|SetMaterial (Variables|Default|GetTL_Human_3wayMirror_RedLight_EM) 0 (select On "/Game/01_Assets/09_TrafficLight/완성예제/material/Light/MI_Emissive_Red.MI_Emissive_Red" "/Game/01_Assets/09_TrafficLight/완성예제/material/Light/M_Emissive_Off.M_Emissive_Off")))

(event EventBeginPlay
  (CallFunction|StartTrafficLight))

(fn ConstructionScript)