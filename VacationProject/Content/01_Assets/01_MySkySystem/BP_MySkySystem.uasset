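; BP_MySkySystem is a sky and weather actor that drives a day cycle and an optional rain state.
; Tick advances TimeOfDay by TimeSpeed and maps it to the directional light's pitch, with SunAngle as yaw.
; The construction script also sets sun rotation, post-process gamma and bloom, rain effect visibility and fog density, where Rainy-based values override FogDensity.
; Rainy drives ripple and rain material parameter collections in both paths.
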(event EventTick
  (params (DeltaSeconds :type Float%20%28single-precision%29))
  (Transformation|SetWorldRotation (Variables|Default|GetDirectionalLight) (Math|Rotator|MakeRotator 0.0 (Math|Float|MapRangeUnclamped (Variables|DirectionalLight|GetTime%20of%20Day) 6e+02 1.8e+03 1.8e+02 3.6e+02) (Variables|DirectionalLight|GetSun%20Angle)) false false)
  (Variables|DirectionalLight|SetTime%20of%20Day (+ (Variables|DirectionalLight|GetTime%20of%20Day) (* DeltaSeconds (Variables|DirectionalLight|GetTime%20Speed))))
  (if (Variables|Default|GetRainy)
    (Rendering|Material|SetScalarParameterValue "/Game/01_Assets/07_RainyWeather/NewMaterialParameterCollection.NewMaterialParameterCollection" "Ripple_Flatten" 0.0 :!class /Script/Engine.KismetMaterialLibrary)
    (Rendering|Material|SetScalarParameterValue "/Game/01_Assets/15_NiagaraEffect/Rain/RainMaterialEffect/MPC_Rain.MPC_Rain" "Rain" 1.0 :!class /Script/Engine.KismetMaterialLibrary)
    (else
      (Rendering|Material|SetScalarParameterValue "/Game/01_Assets/07_RainyWeather/NewMaterialParameterCollection.NewMaterialParameterCollection" "Ripple_Flatten" 1.0 :!class /Script/Engine.KismetMaterialLibrary)
      (Rendering|Material|SetScalarParameterValue "/Game/01_Assets/15_NiagaraEffect/Rain/RainMaterialEffect/MPC_Rain.MPC_Rain" "Rain" 0.0 :!class /Script/Engine.KismetMaterialLibrary))))

(fn ConstructionScript
  (bind _ns_rain (Variables|Default|GetNS_Rain))
  (bind _gamma (Variables|PostProcess|GetGamma))
  (bind _exponentialheightfog (Variables|Default|GetExponentialHeightFog))
  (Utilities|FlowControl|Sequence
    (:then_0
      (Transformation|SetWorldRotation (Variables|Default|GetDirectionalLight) (Math|Rotator|MakeRotator 0.0 (Math|Float|MapRangeUnclamped (Variables|DirectionalLight|GetTime%20of%20Day) 6e+02 1.8e+03 1.8e+02 3.6e+02) (Variables|DirectionalLight|GetSun%20Angle)) false false)
      (Class|ExponentialHeightFogComponent|SetFogDensity (Variables|Default|GetExponentialHeightFog) (Variables|ExponentialHeightFog|GetFog%20Density))
      (Variables|/Script/Engine.PostProcessComponent|SetSettings (Variables|Default|GetPostProcess) (Utilities|Struct|MakePostProcessSettings (Math|Vector4|MakeVector4 _gamma _gamma _gamma 1.0) (Variables|PostProcess|GetBloom%20Intensity))))
    (:then_1
      (if (Variables|Default|GetRainy)
        (Rendering|Material|SetScalarParameterValue "/Game/01_Assets/07_RainyWeather/NewMaterialParameterCollection.NewMaterialParameterCollection" "Ripple_Flatten" 0.0 :!class /Script/Engine.KismetMaterialLibrary)
        (Class|ExponentialHeightFogComponent|SetFogDensity _exponentialheightfog 0.3)
        (Rendering|SetVisibility _ns_rain true false)
        (Rendering|Material|SetScalarParameterValue "/Game/01_Assets/15_NiagaraEffect/Rain/RainMaterialEffect/MPC_Rain.MPC_Rain" "Rain" 1.0 :!class /Script/Engine.KismetMaterialLibrary)
        (else
          (Rendering|Material|SetScalarParameterValue "/Game/01_Assets/07_RainyWeather/NewMaterialParameterCollection.NewMaterialParameterCollection" "Ripple_Flatten" 1.0 :!class /Script/Engine.KismetMaterialLibrary)
          (Class|ExponentialHeightFogComponent|SetFogDensity _exponentialheightfog 0.00381)
          (Rendering|SetVisibility _ns_rain false false)
          (Rendering|Material|SetScalarParameterValue "/Game/01_Assets/15_NiagaraEffect/Rain/RainMaterialEffect/MPC_Rain.MPC_Rain" "Rain" 0.0 :!class /Script/Engine.KismetMaterialLibrary))))))