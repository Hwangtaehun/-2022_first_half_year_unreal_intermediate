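; BP_SplineMeshes builds a chain of deformed meshes along a spline, such as a wire, in its construction script.
; The Wire graph adds spline mesh components using a configurable mesh and two materials.
; SplineMeshVar selects one segment per spline point pair using point tangents, or segments at fixed Spacing along the spline length.
; Spaced segments derive tangents from spline direction scaled by Spacing plus TangentScaleAdd.
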(fn ConstructionScript
  (|Wire))